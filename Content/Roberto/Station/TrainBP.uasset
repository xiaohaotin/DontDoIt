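; Train actor for the Station that slides its Cube toward a target and deals heavy hurt to any BP_Player it hits.
; MoveComponentTo drives the Cube over Speed seconds to a referenced Actor's location, or otherwise to a non-zero Destination, both applied as relative location.
; With AutoMatic on, it departs on BeginPlay, and a Tick-counted timer repeatedly snaps it back to its start and relaunches it.
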(event OnComponentHit(Cube)
  (params (HitComponent :type Primitive%20Component%20Object%20Reference) (OtherActor :type Actor%20Object%20Reference) (OtherComp :type Primitive%20Component%20Object%20Reference) (NormalImpulse :type Vector :default "0, 0, 0") (Hit :type Hit%20Result%20Structure%20%28by%20ref%29))
  (bind _asbp_player (Utilities|Casting|CastToBP_Player OtherActor))
  (Utilities|IsValid _asbp_player
    (:Is%20Valid
      (Class|BPICharacter|Hurt(Message) _asbp_player 1e+02))))

(event Custom|GoToActor
  ;[1 1 1] GOTO_Actor_DESTINATION
  (CallFunction|MoveAT (Transformation|GetActorLocation (Variables|Default|Getactor))))

(event Custom|MoveAT
  (params (NewParam :type Vector))
  ;[1 1 1] Moving
  (Components|MoveComponentTo (Variables|Default|GetCube) NewParam "0, 0, 0" false false (Variables|Default|Getspeed) false))

(event Custom|GoToDetination
  ;[1 1 1] GOTODESTINATION
  (CallFunction|MoveAT (Variables|Default|GetDestination)))

(event EventTick
  (params (DeltaSeconds :type Float%20%28single-precision%29))
  (if (Variables|Default|GetAutoMatic)
    (bind _end (CallFunction|Timer DeltaSeconds))
    (if _end
      (Variables|Default|Setcounter 0.0)
      (CallFunction|TeleportBack)
      (CallFunction|Init))))

(event EventBeginPlay
  ;[1 1 1] Start
  (Variables|Default|SetStartPosition (Variables|/Script/Engine.SceneComponent|GetRelativeLocation (Variables|Default|GetCube)))
  (if (Variables|Default|GetAutoMatic)
    (CallFunction|Init)))

(fn ConstructionScript)

(fn TeleportBack
  (Transformation|SetRelativeLocation (Variables|Default|GetCube) (Variables|Default|GetStartPosition) false false))

(fn Init
  (Utilities|IsValid (Variables|Default|Getactor)
    (:Is%20Valid
      (CallFunction|GotoActor))
    (:Is%20Not%20Valid
      (if (Math|Vector|NotEqual(Vector) (Variables|Default|GetDestination) "0, 0, 0" 0.0001)
        (CallFunction|GotoDetination)))))

(fn Timer
  (params (delta :type Float%20%28single-precision%29))
  (bind _output_get (Variables|Default|Setcounter (+ delta (Variables|Default|Getcounter))))
  (return (>= _output_get (Variables|Default|Gettime))))