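; WaterTrapBP is a water trap that rises while active and hurts the player once it reaches a roof actor.
; Player overlap with Cube or Activate starts the trap; ending overlap stops it.
; Tick grows Cube's Z scale by Speed up to MaxSize, or shrinks it toward StartSize, which is read from X scale, without delta time.
; While growing, HeightCheck sends HurtMessage to the stored player when Top passes Roof.
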(event OnComponentBeginOverlap(Cube)
  (params (OverlappedComponent :type Primitive%20Component%20Object%20Reference) (OtherActor :type Actor%20Object%20Reference) (OtherComp :type Primitive%20Component%20Object%20Reference) (OtherBodyIndex :type Integer) (bFromSweep :type Boolean) (SweepResult :type Hit%20Result%20Structure%20%28by%20ref%29))
  ;[1 1 1] OVERLAP_START_END
  (bind _asbp_player (Utilities|Casting|CastToBP_Player OtherActor))
  (Utilities|IsValid _asbp_player
    (:Is%20Valid
      (Variables|Default|SettrapActive true)
      (Variables|Default|SetPlayer _asbp_player))))

(event OnComponentEndOverlap(Cube)
  (params (OverlappedComponent :type Primitive%20Component%20Object%20Reference) (OtherActor :type Actor%20Object%20Reference) (OtherComp :type Primitive%20Component%20Object%20Reference) (OtherBodyIndex :type Integer))
  ;[1 1 1] OVERLAP_START_END
  (bind _asbp_player (Utilities|Casting|CastToBP_Player OtherActor))
  (Utilities|IsValid _asbp_player
    (:Is%20Valid
      (Variables|Default|SettrapActive false))))

(event Custom|LevelDown
  (bind _cube (Variables|Default|GetCube))
  (bind _speed (Variables|Default|GetSpeed))
  (bind _returnvalue (Transformation|GetWorldScale _cube))
  (bind _returnvalue_2 (- (.z _returnvalue) _speed))
  ;[1 1 1] Deactivation
  (Transformation|SetWorldScale3D _cube (Math|Vector|MakeVector (.x _returnvalue) (.y _returnvalue) _returnvalue_2))
  (Variables|Default|SetCurentSize _returnvalue_2))

(event Custom|LevelUp
  (bind _cube (Variables|Default|GetCube))
  (bind _speed (Variables|Default|GetSpeed))
  (bind _returnvalue (Transformation|GetWorldScale _cube))
  (bind _returnvalue_2 (+ (.z _returnvalue) _speed))
  ;[1 1 1] ACTIVATION
  (Transformation|SetWorldScale3D _cube (Math|Vector|MakeVector (.x _returnvalue) (.y _returnvalue) _returnvalue_2))
  (Variables|Default|SetCurentSize _returnvalue_2))

(event EventBeginPlay
  ;[1 1 1] START
  (bind _output_get (Variables|Default|SetStartSize (.x (Variables|/Script/Engine.SceneComponent|GetRelativeScale3D (Variables|Default|GetCube)))))
  (Variables|Default|SetCurentSize _output_get))

(event EventTick
  (params (DeltaSeconds :type Float%20%28single-precision%29))
  ;[1 1 1] UPDATE
  (if (Variables|Default|GettrapActive)
    (if (< (Variables|Default|GetCurentSize) (Variables|Default|GetMaxSize))
      (CallFunction|LevelUp)
      (CallFunction|HeightCheck))
    (elif (> (Variables|Default|GetCurentSize) (Variables|Default|GetStartSize))
      (CallFunction|LevelDown))))

(fn ConstructionScript)

(fn Activate
  (Variables|Default|SettrapActive true))

(fn HeightCheck
  (bind _player (Variables|Default|GetPlayer))
  (bind _roof (Variables|Default|GetRoof))
  (Utilities|IsValid _roof
    (:Is%20Valid
      (if (> (.z (Transformation|GetWorldLocation (Variables|Default|GetTop))) (.z (Transformation|GetWorldLocation (Variables|/Script/Engine.Actor|GetRootComponent _roof))))
        (Utilities|IsValid _player
          (:Is%20Valid
            (Class|BPICharacter|Hurt(Message) _player 1e+02)))))))