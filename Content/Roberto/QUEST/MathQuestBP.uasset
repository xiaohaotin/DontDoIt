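; MathQuestBP is a math quest that asks random multiplication problems and clears after three correct answers.
; StartQuestion rolls two operands, opens a MathWidget built with them and a self-reference, and switches to UI-only input with the cursor shown.
; CheckResult compares the reply to the product, rerolling on success until the third, when QuestClear removes the widget and restores game input.
; Wrong answers are ignored.
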(event Custom|CheckResult
  (params (Reply :type String))
  ;[1 1 1] CLEARCHECK
  (if (== (Math|Conversions|ToInteger(Byte) Reply) (Variables|Default|Getresult))
    (bind _output_get (Variables|Default|Setclearproblem (+ (Variables|Default|Getclearproblem) 1)))
    (if (>= _output_get 3)
      (CallFunction|QuestClear)
      (Development|PrintString "Congratulation")
      (else
        (CallFunction|RandomProblem)))))

(event Custom|QuestClear
  ;[1 1 1] EndQuest
  (Widget|RemovefromParent (Variables|Default|GetM_Widget))
  (Input|SetInputModeGameOnly (Game|GetPlayerController 0)))

(event Custom|StartQuestion
  (bind _returnvalue (Game|GetPlayerController 0))
  ;[1 1 1] Start
  (CallFunction|RandomProblem)
  (bind _returnvalue_2 (UserInterface|CreateWidget "/Game/Roberto/QUEST/MathWidget.MathWidget_C"))
  (bind _output_get (Variables|Default|SetM_Widget _returnvalue_2))
  (UserInterface|Viewport|AddtoViewport _output_get 0)
  (CallFunction|RandomProblem)
  (Default|BuildProblem (Variables|Default|GetM_Widget) (Variables|Default|GetNum1) (Variables|Default|GetNum2) self)
  (Input|SetInputModeUIOnly _returnvalue (Variables|/Game/Roberto/QUEST/MathWidget.MathWidget_C|GetButton_233 (Variables|Default|GetM_Widget)) "DoNotLock")
  (Variables|/Script/Engine.PlayerController|SetbShowMouseCursor _returnvalue true))

(event Custom|RandomProblem
  ;[1 1 1] MakeRandomProblem
  (bind _output_get (Variables|Default|SetNum1 (Math|Random|RandomIntegerinRange 2 20)))
  (bind _output_get_2 (Variables|Default|SetNum2 (Math|Random|RandomIntegerinRange 2 20)))
  (Variables|Default|Setresult (* _output_get _output_get_2)))

(event EventBeginPlay)

(fn ConstructionScript)