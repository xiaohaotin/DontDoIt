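; Succubus boss enemy that wakes on a toggle event, screaming, waiting, then walking via AI MoveTo to a battle manager point and destroying the mist wall.
; Action events (scream, slash, magic, bite, death) set states on its SUCC_ANIMATOR anim instance.
; TakeDamage lowers HP and flags death, but Death and the Tick death check are empty stubs.
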(event Custom|SetDestination
  (params (pos :type Vector))
  ;[1 1 1] MOVEMENT
  (AI|AIMoveTo (Pawn|GetControlledPawn (Variables|Default|GetController_AI%20)) pos 0 5e+01 false))

(event EventBeginPlay
  ;[1 1 1] START
  (Variables|Default|SetController_AI%20 (AI|GetAIController self))
  (bind _assucc_animator (Utilities|Casting|CastToSUCC_ANIMATOR (Components|SkeletalMesh|GetAnimInstance (Variables|Character|GetMesh))))
  (Variables|Default|SetAnimator _assucc_animator))

(event Collision|EventActorBeginOverlap
  (params (OtherActor :type Actor%20Object%20Reference)))

(event EventTick
  (params (DeltaSeconds :type Float%20%28single-precision%29))
  ;[1 1 1] UPDATE
  (if (Variables|Default|GetisDeath)
    _))

(event EventON/OFFTougle
  (params (boolean :type Boolean))
  (if (not (Variables|Default|Getactive))
    (Variables|Default|Setactive true)
    (CallFunction|Scream)
    (Utilities|FlowControl|Delay 4.0)
    (CallFunction|SetDestination (Variables|/Game/Roberto/Enemy/SUCCUBUS/BossBattleBP.BossBattleBP_C|GetPoint2 (Variables|Default|GetbossBATTLE)))
    (bind _returnvalue (Actor|GetActorOfClass "/Game/Roberto/MistWall.MistWall_C"))
    (Utilities|IsValid _returnvalue
      (:Is%20Valid
        (Default|DestroyWall _returnvalue)))))

(event Custom|Scream
  ;[1 1 1] SCREAM
  (Default|SetState (Variables|Default|GetAnimator) "NewEnumerator4"))

(event Custom|Magic
  ;[1 1 1] MAGIC
  (Default|SetState (Variables|Default|GetAnimator) "NewEnumerator2"))

(event Custom|TwoHandMagic
  ;[1 1 1] MAGIC
  (Default|SetState (Variables|Default|GetAnimator) "NewEnumerator3"))

(event Custom|Slash
  ;[1 1 1] SLASH
  (Default|SetState (Variables|Default|GetAnimator) "NewEnumerator1"))

(event Custom|Bite
  ;[1 1 1] Bite
  (Default|SetState (Variables|Default|GetAnimator) "NewEnumerator6"))

(event Custom|KillSuccubus
  ;[1 1 1] DEATH
  (Default|SetState (Variables|Default|GetAnimator) "NewEnumerator5"))

(fn ConstructionScript)

(fn TakeDamage
  (params (Amount :type Integer))
  (bind _output_get (Variables|Default|SetHP (- (Variables|Default|GetHP) Amount)))
  (bind _output_get_2 (Variables|Default|SetisDeath (<= _output_get 0)))
  (if _output_get_2
    (CallFunction|Death)))

(fn Death)

(fn SetBatleManager
  (params (NewParam :type Boss%20Battle%20BP%20Object%20Reference))
  (Variables|Default|SetbossBATTLE NewParam))