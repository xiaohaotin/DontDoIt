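; Boss battle actor that registers itself with the Succubus enemy in the level.
; On BeginPlay it finds the first SuccubusBP actor and sets that actor's BossBATTLE reference to itself.
; The construction script caches the root component's world location in Point2, which this file never reads.
; A second actor search on BeginPlay has no class shown and its result is unused.
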(event EventBeginPlay
  (bind _outactors (Actor|GetAllActorsOfClass 0))
  (bind _outactors_2 (Actor|GetAllActorsOfClass "/Game/Roberto/Enemy/SUCCUBUS/SuccubusBP.SuccubusBP_C"))
  (bind _output_get (Variables|Default|Setsuccubus (Utilities|Array|Get(acopy) _outactors_2)))
  (Variables|/Game/Roberto/Enemy/SUCCUBUS/SuccubusBP.SuccubusBP_C|SetbossBATTLE _output_get self))

(event Collision|EventActorBeginOverlap
  (params (OtherActor :type Actor%20Object%20Reference)))

(event EventTick
  (params (DeltaSeconds :type Float%20%28single-precision%29)))

(fn ConstructionScript
  (Variables|Default|SetPoint2 (Transformation|GetWorldLocation (Variables|Default|GetDefaultSceneRoot))))