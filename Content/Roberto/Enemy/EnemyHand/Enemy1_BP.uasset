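; Character Blueprint for a hand enemy (Enemy1) that sets up its movement, AI and animation when play begins.
; BeginPlay applies the walk speed and passes the Blueprint's combat, chase and HP stats to Enemy1_AIController through INIT.
; It then caches the mesh's HAND_ANIMATOR anim instance and gives it a reference to that controller.
; Tick and the construction script are empty.
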(event EventBeginPlay
  (Variables|/Script/Engine.CharacterMovementComponent|SetMaxWalkSpeed (Variables|Character|GetCharacterMovement) (Variables|Default|GetwalkSpeed))
  (bind _asenemy_1_aicontroller (Utilities|Casting|CastToEnemy1_AIController (AI|GetAIController self)))
  (Default|INIT _asenemy_1_aicontroller (Variables|Default|GetAtkForce) (Variables|Default|GetAttackRange) (Variables|Default|GetAttackDelay) (Variables|Default|GetchaseDistance) (Variables|Default|GetHP))
  (bind _ashand_animator (Utilities|Casting|CastToHAND_ANIMATOR (Components|SkeletalMesh|GetAnimInstance (Variables|Character|GetMesh))))
  (Variables|Default|SetAnimator _ashand_animator)
  (Variables|/Game/Roberto/Enemy/EnemyHand/Animator/HAND_ANIMATOR.HAND_ANIMATOR_C|SetController (Variables|Default|GetAnimator) _asenemy_1_aicontroller))

(event Collision|EventActorBeginOverlap
  (params (OtherActor :type Actor%20Object%20Reference)))

(event EventTick
  (params (DeltaSeconds :type Float%20%28single-precision%29)))

(fn ConstructionScript)