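; Grenade actor in the Goblin enemy folder that explodes on a timer once thrown.
; Throw only starts the timer and ignores its Destination, so it applies no movement.
; Tick accumulates delta time through CooldownUpdate until Cooldown is reached, then calls Explode.
; Explode spawns the P_Explosion particles and Checkpoint sound at the actor's location and destroys it, with no damage logic.
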(event Custom|Throw
  (params (Destination :type Vector))
  (Variables|Default|SetTimeStart true))

(event EventBeginPlay)

(event Collision|EventActorBeginOverlap
  (params (OtherActor :type Actor%20Object%20Reference)))

(event EventTick
  (params (DeltaSeconds :type Float%20%28single-precision%29))
  (if (Variables|Default|GetTimeStart)
    (bind _timeover (CallFunction|CooldownUpdate DeltaSeconds))
    (if _timeover
      (CallFunction|Explode))))

(fn ConstructionScript)

(fn CooldownUpdate
  (params (delta :type Float%20%28single-precision%29))
  (Variables|Default|SetCurrentTime (+ (Variables|Default|GetCurrentTime) delta))
  (return (>= (Variables|Default|GetCurrentTime) (Variables|Default|GetCooldown))))

(fn Explode
  (bind _returnvalue (Transformation|GetActorLocation))
  (Utilities|FlowControl|Sequence
    (:then_0
      (Effects|SpawnEmitteratLocation "/Game/StarterContent/Particles/P_Explosion.P_Explosion" _returnvalue))
    (:then_1
      (Audio|SpawnSoundatLocation "/Game/Roberto/AudioManager/Music/tracks/checkpoint.checkpoint" _returnvalue "0, 0, 0" 1.0 1.0 0.0 0 0))
    (:then_2
      (Actor|DestroyActor))))