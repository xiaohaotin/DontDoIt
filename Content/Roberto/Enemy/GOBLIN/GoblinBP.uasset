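; GoblinBP is a goblin enemy character that moves under AI control, jumps and throws grenades at the player.
; Movement events send it to a location or target actor through AIMoveTo.
; Jump, death and four directional throw events set a CurrentAction enum.
; ThrowBomb spawns a GranadeBP at an arrow component and throws it at the player's location, looking the player up if needed and falling back to a debug throw.
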(event Custom|SetTargetDestination
  (params (pos :type Actor%20Object%20Reference))
  ;[1 1 1] MOVEMENT
  (AI|AIMoveTo (Pawn|GetControlledPawn (Variables|Default|GetAI)) "0, 0, 0" pos 5e+01 false))

(event Custom|SetDestination
  (params (pos :type Vector))
  ;[1 1 1] MOVEMENT
  (AI|AIMoveTo (Pawn|GetControlledPawn (Variables|Default|GetAI)) pos 0 5e+01 false))

(event EventBeginPlay
  ;[1 1 1] START
  (Variables|Default|SetAI (AI|GetAIController self)))

(event Custom|ThrowRightDown
  (Variables|Default|SetCurrentAction "NewEnumerator6"))

(event Custom|ThrowLeft
  (Variables|Default|SetCurrentAction "NewEnumerator3"))

(event Custom|ThrowRight
  (Variables|Default|SetCurrentAction "NewEnumerator4"))

(event Custom|ThrowLeftDown
  (Variables|Default|SetCurrentAction "NewEnumerator5"))

(fn ConstructionScript)

(fn UseJump
  (Variables|Default|SetCurrentAction "NewEnumerator2")
  (Character|Jump))

(fn Death
  (Variables|Default|SetCurrentAction "NewEnumerator1"))

(fn ThrowBomb
  (Utilities|IsValid (Variables|Default|GetPlayer)
    (:Is%20Valid
      (bind _output_get (LocalVariables|SetDestination (Transformation|GetActorLocation (Variables|Default|GetPlayer)) :!label _label))
      (bind _returnvalue (Game|SpawnActorfromClass "/Game/Roberto/Enemy/GOBLIN/GranadeBP.GranadeBP_C" (Transformation|GetWorldTransform (Variables|Default|GetArrow1)) "AlwaysSpawn" 0 self))
      (bind _output_get_2 (LocalVariables|SetnewBomb _returnvalue))
      (Default|Throw _output_get_2 _output_get))
    (:Is%20Not%20Valid
      (bind _returnvalue_2 (Actor|GetActorOfClass "/Game/OuKanu/Character/BP_Player.BP_Player_C"))
      (bind _output_get_3 (Variables|Default|SetPlayer _returnvalue_2))
      (Utilities|IsValid _output_get_3
        (:Is%20Valid
          (goto _label))
        (:Is%20Not%20Valid
          (CallFunction|DebugBomb))))))

(fn DebugBomb
  (bind _output_get (LocalVariables|SetDestination (* (* (Transformation|GetWorldLocation (Variables|Default|GetArrow1)) (Math|Vector|GetForwardVector "0, 0, 0")) 1e+02)))
  (bind _returnvalue (Game|SpawnActorfromClass "/Game/Roberto/Enemy/GOBLIN/GranadeBP.GranadeBP_C" (Transformation|GetWorldTransform (Variables|Default|GetArrow1)) "AlwaysSpawn" 0 self))
  (bind _output_get_2 (LocalVariables|SetnewBomb _returnvalue))
  (Default|Throw _output_get_2 _output_get))