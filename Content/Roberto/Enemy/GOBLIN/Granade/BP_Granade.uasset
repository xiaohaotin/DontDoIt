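; Goblin grenade actor that is thrown with a physics impulse, then spawns an explosion and destroys itself when its cooldown timer expires.
; The player can grab it, which constrains it, swaps its collision profile and starts a per-tick predicted arc from the player's forward vector.
; A player throw launches it along that arc, or toward the Goblin's mesh if that reference is valid.
; HittingWall also explodes it once it has been grabbed.
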(event Custom|Throw
  (params (Destination :type Vector) (force :type Float%20%28single-precision%29) (NewParam :type Goblin%20BP%20Object%20Reference))
  (bind _staticmesh (Variables|Default|GetStaticMesh))
  ;[1 1 1] THROW
  (Transformation|SetActorScale3D (Variables|Default|GetScale))
  (Variables|Default|SetTimeStart true)
  (Physics|SetSimulatePhysics _staticmesh true)
  (Physics|AddImpulse _staticmesh (* Destination force) "None" false)
  (Variables|Default|Setgoblin 0))

(event EventThrowbyCharacter
  (params (Force :type Vector :default "0, 0, 0"))
  (Utilities|IsValid (Variables|Default|Getgoblin)
    (:Is%20Valid
      (CallFunction|ThrowBack))
    (:Is%20Not%20Valid
      (Physics|SetSimulatePhysics (Variables|Default|GetStaticMesh) true)
      (Physics|AddImpulse (Variables|Default|GetStaticMesh) (Variables|Default|GetDestination) "None" true))))

(event EventTick
  (params (DeltaSeconds :type Float%20%28single-precision%29))
  (bind _returnvalue (Game|Player|GetPlayerPawn 0))
  (bind _rootcomponent (Variables|/Script/Engine.Actor|GetRootComponent _returnvalue))
  ;[1 1 1] COOLDOWN
  (Utilities|FlowControl|Sequence
    (:then_0
      (if (Variables|Default|GetComeBack)
        (bind _output_get (Variables|Default|SetDestination (+ (* (Math|Vector|GetForwardVector _rootcomponent) (Variables|Default|GetForce)) "0, 0,1500.000000")))
        (Class|GameplayStatics|BlueprintPredictProjectilePathbyTraceChannel (Transformation|GetWorldLocation _rootcomponent) _output_get true 1e+01 "ECC_Visibility" false 0 "ForDuration" 0.0)))
    (:then_1
      (if (Variables|Default|GetTimeStart)
        (bind _timeend (CallFunction|CooldownUpdate DeltaSeconds))
        (if _timeend
          (CallFunction|Explode))))))

(event EventDropbyCharacter
  (bind _staticmesh (Variables|Default|GetStaticMesh))
  ;[1 1 1] PICKUP
  (Utilities|FlowControl|Delay 0.2)
  (Class|PrimitiveComponent|SetConstraintMode _staticmesh "Default")
  (Collision|SetCollisionProfileName _staticmesh "PickableitemDefalut" :!class /Script/Engine.PrimitiveComponent))

(event EventGrabbyCharacter
  (params (Grab :type Boolean) (TargetComponent :type Scene%20Component%20Object%20Reference) (MeshComponent :type Mesh%20Component%20Object%20Reference))
  (bind _staticmesh (Variables|Default|GetStaticMesh))
  (bind _staticmesh_2 (Variables|Default|GetStaticMesh))
  ;[1 1 1] PICKUP
  (if Grab
    (Transformation|SetActorLocationAndRotation (Transformation|GetWorldLocation TargetComponent) "0, 0, 0" false true)
    (Class|PrimitiveComponent|SetConstraintMode _staticmesh "XYPlane")
    (Collision|SetCollisionProfileName _staticmesh "PickableitemPicked" :!class /Script/Engine.PrimitiveComponent)
    (Variables|Default|SetComeBack true)
    (else
      (Utilities|FlowControl|Delay 0.2)
      (Class|PrimitiveComponent|SetConstraintMode _staticmesh_2 "Default")
      (Collision|SetCollisionProfileName _staticmesh_2 "PickableitemDefalut" :!class /Script/Engine.PrimitiveComponent))))

(fn ConstructionScript)

(fn CooldownUpdate
  (params (Delta :type Float%20%28single-precision%29))
  (bind _output_get (Variables|Default|SetCounter (+ (Variables|Default|GetCounter) Delta)))
  (return (>= _output_get (Variables|Default|GetCooldownTime))))

(fn Explode
  (Game|SpawnActorfromClass "/Game/Roberto/Enemy/GOBLIN/Granade/ExplosionBP.ExplosionBP_C" (Math|Transform|MakeTransform (Transformation|GetWorldLocation (Variables|Default|GetStaticMesh)) "0, 0, 0" "10.000000,10.000000,10.000000") "Undefined" 0 0)
  (Actor|DestroyActor))

(fn HittingWall
  (if (Variables|Default|GetComeBack)
    (CallFunction|Explode)))

(fn ThrowBack
  (Physics|SetSimulatePhysics (Variables|Default|GetStaticMesh) true)
  (Physics|AddImpulse (Variables|Default|GetStaticMesh) (* (- (Transformation|GetWorldLocation (Variables|/Script/Engine.Character|GetMesh (Variables|Default|Getgoblin))) (Transformation|GetWorldLocation (Variables|Default|GetStaticMesh))) 1e+01) "None" true))

(fn GetGrabBox
  (return 0))

(fn GetHintButtonIcon
  (return "NewEnumerator0"))

(fn GetHintUIText
  (return ""))

(fn GetItemType
  (return "NewEnumerator0"))

(fn GetRope
  (return 0))