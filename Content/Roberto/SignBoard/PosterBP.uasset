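; Poster sign actor that fades out and hides once a BP_Character enters its trigger box.
; BeginPlay puts a dynamic instance of PosterMat on the skeletal mesh at full alpha, and the overlap sets an Activate flag.
; While active, Tick adds Speed to a counter and Clear writes Unit minus the counter into the Alpha vector parameter, hiding the mesh at zero.
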(event OnComponentBeginOverlap(Box)
  (params (OverlappedComponent :type Primitive%20Component%20Object%20Reference) (OtherActor :type Actor%20Object%20Reference) (OtherComp :type Primitive%20Component%20Object%20Reference) (OtherBodyIndex :type Integer) (bFromSweep :type Boolean) (SweepResult :type Hit%20Result%20Structure%20%28by%20ref%29))
  (bind _asbp_character (Utilities|Casting|CastToBP_Character OtherActor))
  (Utilities|IsValid _asbp_character
    (:Is%20Valid
      (Variables|Default|Setactivate true))))

(event EventTick
  (params (DeltaSeconds :type Float%20%28single-precision%29))
  (if (Variables|Default|Getactivate)
    (Variables|Default|Setcounter (+ (Variables|Default|Getcounter) (Variables|Default|Getspeed)))
    (CallFunction|Clear)))

(event EventBeginPlay
  (bind _returnvalue (Rendering|Material|CreateDynamicMaterialInstance "/Game/Roberto/SignBoard/Materials/PosterMat.PosterMat" "None" :!class /Script/Engine.KismetMaterialLibrary))
  (bind _output_get (Variables|Default|SetMat _returnvalue))
  (Rendering|Material|SetMaterial (Variables|Default|GetSkeletalMesh) 0 _output_get)
  (Rendering|Material|SetVectorParameterValue (Variables|Default|GetMat) (Variables|Default|GetAlpha) (Utilities|Struct|MakeLinearColor 1.0 1.0 1.0 1.0) :!class /Script/Engine.MaterialInstanceDynamic))

(fn ConstructionScript)

(fn Clear
  (bind _unit (Variables|Default|GetUnit))
  (bind _counter (Variables|Default|Getcounter))
  (bind _returnvalue (- _unit _counter))
  (if (<= _returnvalue 0.0)
    (Variables|Default|Setactivate false)
    (Rendering|Material|SetVectorParameterValue (Variables|Default|GetMat) (Variables|Default|GetAlpha) (Utilities|Struct|MakeLinearColor 1.0 1.0 1.0 0.0) :!class /Script/Engine.MaterialInstanceDynamic)
    (Rendering|SetVisibility (Variables|Default|GetSkeletalMesh) false false)
    (else
      (Rendering|Material|SetVectorParameterValue (Variables|Default|GetMat) (Variables|Default|GetAlpha) (Utilities|Struct|MakeLinearColor 1.0 1.0 1.0 _returnvalue) :!class /Script/Engine.MaterialInstanceDynamic))))