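; Checkpoint actor that saves or clears the player's respawn state when anything begins overlapping its Trigger.
; With its Load flag on, it writes player 0's location and a load flag to the "check" save slot through BP_SaveTheGame, creating the save if missing, then destroys itself after a short delay.
; With Load off, it sets the saved flag to false and stays in place.
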(event OnComponentBeginOverlap(Trigger)
  (params (OverlappedComponent :type Primitive%20Component%20Object%20Reference) (OtherActor :type Actor%20Object%20Reference) (OtherComp :type Primitive%20Component%20Object%20Reference) (OtherBodyIndex :type Integer) (bFromSweep :type Boolean) (SweepResult :type Hit%20Result%20Structure%20%28by%20ref%29))
  (if (Variables|Default|GetLoad)
    (Utilities|FlowControl|Sequence
      (:then_0
        (bind _ascharacter (Utilities|Casting|CastToCharacter (Game|GetPlayerCharacter 0)))
        (Variables|Default|SetPlayerLoc (Transformation|GetActorLocation _ascharacter))
        (Development|PrintString "CheckPoint Recheck"))
      (:then_1
        (bind _returnvalue (SaveGame|DoesSaveGameExist "check"))
        (if _returnvalue
          (bind _returnvalue_2 (SaveGame|LoadGamefromSlot "check"))
          (bind _asbp_save_the_game (Utilities|Casting|CastToBP_SaveTheGame _returnvalue_2))
          (Variables|/Game/XiaoHaoTing/BP_SaveTheGame.BP_SaveTheGame_C|SetPlayer_locals _asbp_save_the_game (Variables|Default|GetPlayerLoc))
          (Variables|/Game/XiaoHaoTing/BP_SaveTheGame.BP_SaveTheGame_C|SetLoad _asbp_save_the_game true)
          (SaveGame|SaveGametoSlot _asbp_save_the_game "check")
          (else
            (bind _returnvalue_3 (SaveGame|CreateSaveGameObject "/Game/XiaoHaoTing/BP_SaveTheGame.BP_SaveTheGame_C"))
            (Variables|/Game/XiaoHaoTing/BP_SaveTheGame.BP_SaveTheGame_C|SetPlayer_locals _returnvalue_3 (Variables|Default|GetPlayerLoc))
            (Variables|/Game/XiaoHaoTing/BP_SaveTheGame.BP_SaveTheGame_C|SetLoad _returnvalue_3 true)
            (SaveGame|SaveGametoSlot _returnvalue_3 "check")))
        (Utilities|FlowControl|Delay 2.0)
        (Actor|DestroyActor)))
    (else
      (bind _returnvalue_4 (SaveGame|LoadGamefromSlot "check"))
      (bind _asbp_save_the_game_2 (Utilities|Casting|CastToBP_SaveTheGame _returnvalue_4))
      (Variables|/Game/XiaoHaoTing/BP_SaveTheGame.BP_SaveTheGame_C|SetLoad _asbp_save_the_game_2 false)
      (SaveGame|SaveGametoSlot _asbp_save_the_game_2 "check")
      (Development|PrintString "CheckPoint Clear"))))

(event EventBeginPlay)

(event Collision|EventActorBeginOverlap
  (params (OtherActor :type Actor%20Object%20Reference)))

(event EventTick
  (params (DeltaSeconds :type Float%20%28single-precision%29)))

(fn ConstructionScript)