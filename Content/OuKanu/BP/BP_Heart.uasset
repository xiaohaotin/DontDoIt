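; BP_Heart is a health pickup that heals a living player on touch.
; Its sphere overlap checks player and death state through message calls, sends HealMessage with the HPRecover amount, then plays a particle and sound and destroys itself.
; A custom event restarts the SelfRotation timeline, which drives the heart's height and yaw from one vector track; nothing in this file calls that event.
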(event OnComponentBeginOverlap(Sphere)
  (params (OverlappedComponent :type Primitive%20Component%20Object%20Reference) (OtherActor :type Actor%20Object%20Reference) (OtherComp :type Primitive%20Component%20Object%20Reference) (OtherBodyIndex :type Integer) (bFromSweep :type Boolean) (SweepResult :type Hit%20Result%20Structure%20%28by%20ref%29))
  (bind _yes_no (Class|BPIPlayer|IsPlayer(Message) OtherActor))
  (if _yes_no
    (bind _isdead (Class|BPICharacter|GetIsDead(Message) OtherActor))
    (if (not _isdead)
      (Class|BPICharacter|Heal(Message) OtherActor (Variables|Default|GetHPRecover) false)
      (CallFunction|PlayConsumedFX)
      (Actor|DestroyActor))))

(event Custom|Event_ResetSelfRotation
  (bind _height_rotaton (Timeline|SelfRotation PlayFromStart)
    (:Update
      (Transformation|SetRelativeLocationAndRotation (Variables|Default|Getheart) (Math|Vector|MakeVector 0.0 0.0 (.X (Math|Vector|BreakVector _height_rotaton))) (Math|Rotator|MakeRotator 0.0 0.0 (.Y (Math|Vector|BreakVector _height_rotaton))) false false))))

(event Custom|PlayConsumedFX
  (bind _heart (Variables|Default|Getheart))
  (bind _returnvalue (Transformation|GetWorldLocation _heart))
  ;[1 1 1] Particle
  (Effects|SpawnEmitteratLocation "/Game/OuKanu/FX/FXVarietyPack/Particles/P_ky_waterBallHit.P_ky_waterBallHit" _returnvalue)
  ;[1 1 1] Sound
  (Audio|PlaySoundatLocation "/Game/Roberto/AudioManager/Music/SFX_Cue/checkpoint_Cue.checkpoint_Cue" _returnvalue "0, 0, 0" 1.0 1.0 0.0 0 0 0))

(event EventBeginPlay)

(event EventTick
  (params (DeltaSeconds :type Float%20%28single-precision%29)))

(fn ConstructionScript)