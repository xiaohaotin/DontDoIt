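; BP_Gateway is a two-sided gate actor that opens and closes as the player passes its trigger volumes.
; Overlapping Enter sets Open and makes BlockBox ignore the Pawn channel, while overlapping Exit clears it and restores blocking.
; Both triggers respond only to actors that pass the IsPlayerMessage check.
; SyncGateWayAnim then forwards the Open state to the left and right gateway anim instances through ToggleEnableMessage.
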(event OnComponentBeginOverlap(Enter)
  (params (OverlappedComponent :type Primitive%20Component%20Object%20Reference) (OtherActor :type Actor%20Object%20Reference) (OtherComp :type Primitive%20Component%20Object%20Reference) (OtherBodyIndex :type Integer) (bFromSweep :type Boolean) (SweepResult :type Hit%20Result%20Structure%20%28by%20ref%29))
  (bind _yes_no (Class|BPIPlayer|IsPlayer(Message) OtherActor))
  (if _yes_no
    (Variables|Default|SetOpen true)
    (Collision|SetCollisionResponsetoChannel (Variables|Default|GetBlockBox) "ECC_Pawn" "ECR_Ignore")
    (CallFunction|SyncGateWayAnim)))

(event OnComponentBeginOverlap(Exit)
  (params (OverlappedComponent :type Primitive%20Component%20Object%20Reference) (OtherActor :type Actor%20Object%20Reference) (OtherComp :type Primitive%20Component%20Object%20Reference) (OtherBodyIndex :type Integer) (bFromSweep :type Boolean) (SweepResult :type Hit%20Result%20Structure%20%28by%20ref%29))
  (bind _yes_no (Class|BPIPlayer|IsPlayer(Message) OtherActor))
  (if _yes_no
    (Variables|Default|SetOpen false)
    (Collision|SetCollisionResponsetoChannel (Variables|Default|GetBlockBox) "ECC_Pawn" "ECR_Block")
    (CallFunction|SyncGateWayAnim)))

(event Custom|SyncGateWayAnim
  (bind _open (Variables|Default|GetOpen))
  (Class|BPIBinaryState|ToggleEnable(Message) (Components|SkeletalMesh|GetAnimInstance (Variables|Default|GetGatewayLeft)) _open)
  (Class|BPIBinaryState|ToggleEnable(Message) (Components|SkeletalMesh|GetAnimInstance (Variables|Default|GetGatewayRight)) _open))

(event EventBeginPlay)

(event Collision|EventActorBeginOverlap
  (params (OtherActor :type Actor%20Object%20Reference)))

(event EventTick
  (params (DeltaSeconds :type Float%20%28single-precision%29)))

(fn ConstructionScript)