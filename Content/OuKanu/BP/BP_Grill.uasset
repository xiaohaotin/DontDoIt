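; BP_Grill is a grill prop that can be knocked loose with physics and restored to its original position.
; BeginPlay caches the Grill component's relative transform.
; Fall enables physics simulation and applies a strong upward impulse at the Scene component's location.
; Reset disables physics, reattaches Grill to Scene, since simulation detaches it, and reapplies the cached transform.
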(event Custom|Fall
  (Physics|SetSimulatePhysics (Variables|Default|GetGrill) true)
  (Physics|AddImpulseatLocation (Variables|Default|GetGrill) "0, 0,50000.000000" (Transformation|GetWorldLocation (Variables|Default|GetScene)) "None"))

(event Custom|Reset
  (Physics|SetSimulatePhysics (Variables|Default|GetGrill) false)
  (Transformation|AttachComponentToComponent (Variables|Default|GetGrill) (Variables|Default|GetScene) "None" "KeepRelative" "KeepRelative" "KeepRelative" true)
  (Transformation|SetRelativeTransform (Variables|Default|GetGrill) (Variables|Default|GetStartTrans) false false))

(event EventBeginPlay
  (Variables|Default|SetStartTrans (Transformation|GetRelativeTransform (Variables|Default|GetGrill))))

(event Collision|EventActorBeginOverlap
  (params (OtherActor :type Actor%20Object%20Reference)))

(event EventTick
  (params (DeltaSeconds :type Float%20%28single-precision%29)))

(fn ConstructionScript)