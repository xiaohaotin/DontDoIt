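; Boss battle item manager that repositions the Mirror item whenever it is destroyed with a "boomed" event.
; On BeginPlay it binds to the Mirror's MirrorBoomed event.
; When that fires, it walks the SpawnPoints array in order and teleports the existing Mirror's BoxCollider to the first point without a player in it, rather than spawning a new actor.
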(event Custom|SpawnMirrorAtPoint
  (bind _spawnpoints (Variables|Mirror|GetSpawnPoints))
  (bind _index (Utilities|FlowControl|ForLoopwithBreak 0 (- (Utilities|Array|Length _spawnpoints) 1) :!label _label)
    (:LoopBody
      (if (not (Variables|/Game/OuKanu/BP/BossBottleUtility/BP_XNORPlayerPoint.BP_XNORPlayerPoint_C|GetPlayerIn (Utilities|Array|Get(acopy) _spawnpoints _index)))
        (Transformation|SetWorldLocation (Variables|/Game/OuKanu/InteractableObject/MirrorSet/BP_MirrorModel.BP_MirrorModel_C|GetBoxCollider (Variables|Mirror|GetMirror)) (Transformation|GetWorldLocation (Variables|/Game/OuKanu/BP/BossBottleUtility/BP_XNORPlayerPoint.BP_XNORPlayerPoint_C|GetDefaultSceneRoot (Utilities|Array|Get(acopy) _spawnpoints _index))) false true)
        (goto _label Break)))))

(event Custom|OnMirrorBoomed
  (CallFunction|SpawnMirroratPoint))

(event EventBeginPlay
  (EventDispatchers|BindEventtoMirrorBoomed (Variables|Mirror|GetMirror) (delegate Custom|OnMirrorBoomed)))

(event Collision|EventActorBeginOverlap
  (params (OtherActor :type Actor%20Object%20Reference)))

(event EventTick
  (params (DeltaSeconds :type Float%20%28single-precision%29)))

(fn ConstructionScript)