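; BP_GrandFather is the grandfather character, which walks to a target point when the player enters its trigger.
; BeginPlay converts TargetPoint from an offset relative to the actor's location into a world position.
; Trigger overlap identifies the player through an IsPlayer message, then calls WalkToPoint to issue an AI MoveTo.
; StartMove is set as soon as the move is issued, not on arrival, so later overlaps do not restart it.
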(event OnComponentBeginOverlap(Trigger)
  (params (OverlappedComponent :type Primitive%20Component%20Object%20Reference) (OtherActor :type Actor%20Object%20Reference) (OtherComp :type Primitive%20Component%20Object%20Reference) (OtherBodyIndex :type Integer) (bFromSweep :type Boolean) (SweepResult :type Hit%20Result%20Structure%20%28by%20ref%29))
  (bind _yes_no (Class|BPIPlayer|IsPlayer(Message) OtherActor))
  (if _yes_no
    (CallFunction|WalktoPoint)))

(event Custom|WalkToPoint
  (if (not (Variables|Default|GetStartMove))
    (AI|AIMoveTo (Pawn|GetController) self (Variables|Default|GetTargetPoint) 0 5.0 true
      (:then
        (Variables|Default|SetStartMove true)))))

(event EventBeginPlay
  ;[1 1 1] Convert to World
  (Variables|Default|SetTargetPoint (+ (Transformation|GetActorLocation) (Variables|Default|GetTargetPoint))))

(event Collision|EventActorBeginOverlap
  (params (OtherActor :type Actor%20Object%20Reference)))

(event EventTick
  (params (DeltaSeconds :type Float%20%28single-precision%29)))

(fn ConstructionScript)