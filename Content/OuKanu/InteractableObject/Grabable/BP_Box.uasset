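; BP_Box is an interactable box whose hint tells the player it can be climbed or grabbed.
; Grab events nudge the box mesh up one unit when grabbed and back down when released or dropped, without sweeping.
; Getter functions expose the box itself as the grab target, plus its hint icon, hint text and item type; the rope getter returns nothing.
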(event EventBeginPlay)

(event Collision|EventActorBeginOverlap
  (params (OtherActor :type Actor%20Object%20Reference)))

(event EventTick
  (params (DeltaSeconds :type Float%20%28single-precision%29)))

(event EventGrabbyCharacter
  (params (Grab :type Boolean) (TargetComponent :type Scene%20Component%20Object%20Reference) (MeshComponent :type Mesh%20Component%20Object%20Reference))
  (bind _boxmesh (Variables|Default|Getboxmesh))
  (bind _boxmesh_2 (Variables|Default|Getboxmesh))
  (if Grab
    (Transformation|SetWorldLocation _boxmesh (+ (Transformation|GetWorldLocation _boxmesh) "0, 0,1.000000") false false)
    (else
      (Transformation|SetWorldLocation _boxmesh_2 (+ (Transformation|GetWorldLocation _boxmesh_2) "0, 0,-1.000000") false false))))

(event EventDropbyCharacter
  (bind _boxmesh (Variables|Default|Getboxmesh))
  (Transformation|SetWorldLocation _boxmesh (+ (Transformation|GetWorldLocation _boxmesh) "0, 0,-1.000000") false false))

(fn ConstructionScript)

(fn GetGrabBox
  (return self))

(fn GetHintButtonIcon
  (return "NewEnumerator10"))

(fn GetHintUIText
  (return "Press \"Space/A\" To Climb 
Press \"RightMouse/R2\"To Grab"))

(fn GetItemType
  (return "NewEnumerator1"))

(fn GetRope
  (return 0))