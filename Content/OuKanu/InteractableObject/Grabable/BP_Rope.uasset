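; BP_Rope is a grabbable rope that exposes grab state, hint and launch data through interface-style functions.
; The GrabbyCharacter event stores the grab flag, while getters return the rope itself, item type, hint icon and "Space/A" prompt.
; Launch direction is the normalized horizontal vector from RopeTop to Sphere, ignoring height.
; It always reports ready to be grabbed, and GetGrabBox returns no value.
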(event EventBeginPlay)

(event Collision|EventActorBeginOverlap
  (params (OtherActor :type Actor%20Object%20Reference)))

(event EventGrabbyCharacter
  (params (Grab :type Boolean) (TargetComponent :type Scene%20Component%20Object%20Reference) (MeshComponent :type Mesh%20Component%20Object%20Reference))
  (Variables|Default|SetIsGrabbed Grab))

(fn ConstructionScript)

(fn GetLaunchDirectionN
  (bind _ropetop (Variables|Default|GetRopeTop))
  (bind _sphere (Variables|Default|GetSphere))
  (bind _returnvalue (Transformation|GetWorldLocation _ropetop))
  (bind _returnvalue_2 (Transformation|GetWorldLocation _sphere))
  (bind (_x _y) (Math|Vector|BreakVector _returnvalue_2))
  (bind (_x_2 _y_2) (Math|Vector|BreakVector _returnvalue))
  (return (Math|Vector|Normalize (Math|Vector|MakeVector (- _x _x_2) (- _y _y_2) 0.0))))

(fn GetGrabBox
  (return 0))

(fn GetHintButtonIcon
  (return "NewEnumerator1"))

(fn GetHintUIText
  (return "Press \"Space/A\" To Grab"))

(fn GetItemType
  (return "NewEnumerator2"))

(fn GetRope
  (return self))

(fn IsGrabbed?
  (return (Variables|Default|GetIsGrabbed)))

(fn ReadytobeGrabbed?
  (return true))