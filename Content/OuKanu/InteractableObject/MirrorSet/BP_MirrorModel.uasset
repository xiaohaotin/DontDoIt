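; BP_MirrorModel is a grabbable mirror item that players carry and place on pedestals, with a check for laser hits.
; Grabbing attaches it to the character with collision off; dropping moves it to any assigned pedestal and restores collision.
; IFFacingLaser rejects back-side hits via dot product and returns the normal, while AddEmmisive boosts a material glow that decays each Tick.
; DestructItem detaches it, spawns an explosion and fires CallMirrorBoomed for the item manager to relocate it.
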(event EventBeginPlay
  (bind _mirror_staticmesh (Variables|Default|GetMirror_StaticMesh))
  (bind _returnvalue (Rendering|Material|CreateDynamicMaterialInstance _mirror_staticmesh 1 (Rendering|Material|GetMaterial _mirror_staticmesh 1) "None" :!class /Script/Engine.PrimitiveComponent))
  (Variables|Default|SetMaterialInst _returnvalue))

(event Collision|EventActorBeginOverlap
  (params (OtherActor :type Actor%20Object%20Reference)))

(event EventTick
  (params (DeltaSeconds :type Float%20%28single-precision%29))
  (bind _output_get (Variables|Default|SetEmmisivePower (Math|Float|Clamp(Float) (- (Variables|Default|GetEmmisivePower) 0.15) 0.1 1e+01)))
  (Rendering|Material|SetScalarParameterValue (Variables|Default|GetMaterialInst) "EmmsivePow" _output_get :!class /Script/Engine.MaterialInstanceDynamic))

(event EventGrabbyCharacter
  (params (Grab :type Boolean) (TargetComponent :type Scene%20Component%20Object%20Reference) (MeshComponent :type Mesh%20Component%20Object%20Reference))
  (if Grab
    (Variables|Default|SetPedestal 0)
    (bind _asbp_character (Utilities|Casting|CastToBP_Character (Components|GetOwner TargetComponent)))
    (bind _output_get (Variables|Default|SetHolder _asbp_character))
    (Transformation|AttachActorToActor _output_get "None" "KeepWorld" "KeepWorld" "KeepWorld" true)
    (Collision|SetCollisionEnabled (Variables|Default|GetMirror_StaticMesh) "NoCollision")
    (Variables|Default|SetPossessedByPlayer true)
    (Class|BPIPlayer|ToggleHintUI(Message) (Variables|Default|GetHolder) "" "NewEnumerator0" false)
    (Components|MoveComponentTo (Variables|Default|GetBoxCollider) "42.000000, 0,30.000000" "0, 0, 0" false false 0.2 false)
    (else
      (CallFunction|DropbyCharacter))))

(event EventSetPedestal
  (params (Pedestal :type Actor%20Object%20Reference))
  (bind _asbp_pedestal (Utilities|Casting|CastToBP_Pedestal Pedestal)
    (:then
      (Variables|Default|SetPedestal _asbp_pedestal))
    (:CastFailed
      (Variables|Default|SetPedestal 0))))

(event EventAddEmmisive
  (Variables|Default|SetEmmisivePower (+ (Variables|Default|GetEmmisivePower) 0.3)))

(event EventDestructItem
  (Variables|Default|SetHolder 0)
  (Variables|Default|SetPossessedByPlayer false)
  (Transformation|DetachFromActor "KeepWorld" "KeepWorld" "KeepWorld")
  (Effects|SpawnEmitteratLocation "/Game/StarterContent/Particles/P_Explosion.P_Explosion" (Transformation|GetActorLocation))
  (Collision|SetCollisionEnabled (Variables|Default|GetMirror_StaticMesh) "QueryAndPhysics")
  ;[1 1 1] Tell Item manager to Move This Mirror
  (Default|CallMirrorBoomed))

(event EventDropbyCharacter
  (bind _pedestal (Variables|Default|GetPedestal))
  (Transformation|DetachFromActor "KeepWorld" "KeepWorld" "KeepWorld")
  (Variables|Default|SetHolder 0)
  (Variables|Default|SetPossessedByPlayer false)
  (Utilities|FlowControl|Sequence
    (:then_0
      ;[1 1 1] If Find Pedestal
      (Utilities|IsValid _pedestal
        (:Is%20Valid
          ;[1 1 1] MoveMirrorToPedestal
          (Transformation|AttachComponentToComponent (Variables|/Game/OuKanu/InteractableObject/MirrorSet/BP_Pedestal.BP_Pedestal_C|GetMirrorPos _pedestal) "None" "KeepWorld" "KeepWorld" "KeepWorld" true)
          (Components|MoveComponentTo (Variables|Default|GetBoxCollider) "0, 0, 0" "0, 0, 0" false false 0.2 false)
          (Transformation|DetachFromComponent (Variables|Default|GetBoxCollider) "KeepWorld" "KeepWorld" "KeepWorld" true))))
    (:then_1
      ;[1 1 1] EnableCollision
      (Collision|SetCollisionEnabled (Variables|Default|GetMirror_StaticMesh) "QueryAndPhysics"))))

(fn ConstructionScript)

(fn GetGrabBox
  (return 0))

(fn GetHintButtonIcon
  (bind _isgrabbed (CallFunction|IsGrabbed?))
  (if _isgrabbed
    (return "NewEnumerator0")
    (else
      (return "NewEnumerator10"))))

(fn GetHintUIText
  (return ""))

(fn GetItemType
  (return "NewEnumerator4"))

(fn GetRope
  (return 0))

(fn IFFacingLaser
  (params (LaserDirection :type Vector :default "0, 0, 0"))
  (bind _mirror_staticmesh (Variables|Default|GetMirror_StaticMesh))
  (bind _returnvalue (Transformation|GetWorldRotation _mirror_staticmesh))
  (bind _returnvalue_2 (Math|Vector|GetRightVector _returnvalue))
  (return (< (Math|Vector|DotProduct LaserDirection _returnvalue_2) 0.0) _returnvalue_2))

(fn IsGrabbed?
  (return (Variables|Default|GetPossessedByPlayer)))

(fn ReadytobeGrabbed?
  (return true))