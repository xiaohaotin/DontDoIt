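; BP_Charger is an interactable battery charger that switches an assigned Platform on or off.
; ToggleActive stores the state, forwards it to the Platform, and updates a particle effect's visibility to match, printing an error if no Platform is assigned.
; Getter functions expose the CharacterPos component and its transforms, plus the BatteryPos world transform through GetMirrorPosWorldTrans.
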(event Custom|ToggleActive
  (params (Enable :type Boolean))
  (bind _platform (Variables|Default|GetPlatform))
  (bind _particlesystem (Variables|Default|GetParticleSystem))
  (bind _output_get (Variables|Default|SetIsActivate Enable))
  (Utilities|IsValid _platform
    (:Is%20Valid
      (Default|ToggleActive _platform _output_get)
      (Components|Activation|Activate _particlesystem false)
      (Rendering|SetVisibility _particlesystem _output_get false))
    (:Is%20Not%20Valid
      (Development|PrintString "Error! Please Assign Platform In Editor" true true "(R=1.000000,G=0.000000,B=0.000000,A=1.000000)"))))

(event EventBeginPlay)

(event Collision|EventActorBeginOverlap
  (params (OtherActor :type Actor%20Object%20Reference)))

(event EventTick
  (params (DeltaSeconds :type Float%20%28single-precision%29)))

(fn ConstructionScript)

(fn GetCharacterPosComponent
  (return (Variables|Default|GetCharacterPos)))

(fn GetCharacterPosRelativeTrans
  (return (Transformation|GetRelativeTransform (Variables|Default|GetCharacterPos))))

(fn GetCharacterPosWorldTrans
  (return (Transformation|GetWorldTransform (Variables|Default|GetCharacterPos))))

(fn GetMirrorPosWorldTrans
  (return (Transformation|GetWorldTransform (Variables|Default|GetBatteryPos))))