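; BP_Battery is a grabbable puzzle item that the character carries to power a BP_Charger.
; Grabbing attaches it to the character and deactivates its current charger.
; Dropping either moves it onto the charger assigned through SetPedestal and activates it, or lowers it by a fixed offset, with a short re-grab delay.
; On a level phase reset, it drops and returns to its start location unless a charger is assigned.
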(event Custom|ResetPosition
  ;[1 1 1] Save & Load
  (Transformation|SetWorldLocation (Variables|Default|GetBatteryMesh) (Variables|Default|GetStartLocation) false false)
  (Variables|Default|SetIsReady true))

(event Custom|Level_ResetCurrentPhase_Event_0
  ;[1 1 1] Save & Load
  ;;[1 1 1] Keep State If Activate A Charger
  (Utilities|IsValid (Variables|Default|GetCharger)
    (:Is%20Not%20Valid
      (CallFunction|DropbyCharacter)
      (CallFunction|ResetPosition))))

(event EventBeginPlay
  ;[1 1 1] Save & Load
  (Variables|Default|SetStartLocation (Transformation|GetWorldLocation (Variables|Default|GetBatteryMesh)))
  (bind _asplayer_controller_custom (Utilities|Casting|CastToPlayerController_Custom (Game|GetPlayerController 0)))
  (EventDispatchers|AssignLevelResetCurrentPhase _asplayer_controller_custom (delegate Custom|Level_ResetCurrentPhase_Event_0)))

(event EventSetPedestal
  (params (Pedestal :type Actor%20Object%20Reference))
  (bind _asbp_charger (Utilities|Casting|CastToBP_Charger Pedestal)
    (:then
      (Variables|Default|SetCharger _asbp_charger))
    (:CastFailed
      (Variables|Default|SetCharger 0))))

(event EventGrabbyCharacter
  (params (Grab :type Boolean) (TargetComponent :type Scene%20Component%20Object%20Reference) (MeshComponent :type Mesh%20Component%20Object%20Reference))
  (if Grab
    (Utilities|IsValid (Variables|Default|GetCharger)
      (:Is%20Valid
        (Default|ToggleActive (Variables|Default|GetCharger) false)
        (Variables|Default|SetCharger 0))
      (:Is%20Not%20Valid
        _))
    (bind _asbp_character (Utilities|Casting|CastToBP_Character (Components|GetOwner TargetComponent)))
    (Transformation|AttachActorToActor _asbp_character "None" "KeepWorld" "KeepWorld" "KeepWorld" true)
    (Variables|Default|SetIsGrabbed true)
    (Variables|Default|SetIsReady false)
    (Components|MoveComponentTo (Variables|Default|GetBatteryMesh) "42.000000, 0,30.000000" "0, 0, 0" false false 0.2 false)
    (else
      (CallFunction|DropbyCharacter))))

(event EventDropbyCharacter
  (bind _charger (Variables|Default|GetCharger))
  (Transformation|DetachFromActor "KeepWorld" "KeepWorld" "KeepWorld")
  (Variables|Default|SetHolder 0)
  (Utilities|FlowControl|Sequence
    (:then_0
      (Variables|Default|SetIsGrabbed false)
      (Utilities|FlowControl|Delay 0.5)
      (Variables|Default|SetIsReady true))
    (:then_1
      ;[1 1 1] If Find Pedestal
      (Utilities|IsValid _charger
        (:Is%20Valid
          ;[1 1 1] MoveBatteryToPedestal
          (Transformation|AttachComponentToComponent (Variables|/Game/OuKanu/InteractableObject/BatterySet/BP_Charger.BP_Charger_C|GetBatteryPos _charger) "None" "KeepWorld" "KeepWorld" "KeepWorld" true)
          (Components|MoveComponentTo (Variables|Default|GetBatteryMesh) "0, 0, 0" "0, 0, 0" false false 0.2 true)
          (Transformation|DetachFromComponent (Variables|Default|GetBatteryMesh) "KeepWorld" "KeepWorld" "KeepWorld" true)
          (Default|ToggleActive (Variables|Default|GetCharger) true))
        (:Is%20Not%20Valid
          ;[1 1 1] Move To Ground
          (Transformation|AddActorWorldOffset "0, 0,-128.000000"))))))

(fn ConstructionScript)

(fn GetGrabBox
  (return 0))

(fn GetHintButtonIcon
  (return "NewEnumerator10"))

(fn GetHintUIText
  (return ""))

(fn GetItemType
  (return "NewEnumerator5"))

(fn GetRope
  (return 0))

(fn IFFacingLaser
  (params (LaserDirection :type Vector :default "0, 0, 0"))
  (return false "0, 0, 0"))

(fn IsGrabbed?
  (return (Variables|Default|GetIsGrabbed)))

(fn ReadytobeGrabbed?
  (return (Variables|Default|GetIsReady)))