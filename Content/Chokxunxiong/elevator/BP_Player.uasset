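; Player character Blueprint handling health feedback, hint text, death and checkpoint respawn.
; HP updates the controller-provided bar, and lost health gradually shortens the spring arm; overlaps show hint text, and falling below kill height deals massive damage.
; Death fades the screen via MP_Player parameters and the GameMode, plays a montage, ragdolls, then requests checkpoint respawn.
; Rebirth undoes the ragdoll, heals, resets the camera and replays the start bloom.
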(event OnComponentBeginOverlap(HintUIBox)
  (params (OverlappedComponent :type Primitive%20Component%20Object%20Reference) (OtherActor :type Actor%20Object%20Reference) (OtherComp :type Primitive%20Component%20Object%20Reference) (OtherBodyIndex :type Integer) (bFromSweep :type Boolean) (SweepResult :type Hit%20Result%20Structure%20%28by%20ref%29))
  ;[0.08121 1 0.1267] Hint UI Check
  (bind _text (Class|BPIItem|GetHintUIText(Message) OtherActor))
  (CallFunction|ToggleHintUI _text true))

(event OnComponentEndOverlap(HintUIBox)
  (params (OverlappedComponent :type Primitive%20Component%20Object%20Reference) (OtherActor :type Actor%20Object%20Reference) (OtherComp :type Primitive%20Component%20Object%20Reference) (OtherBodyIndex :type Integer))
  ;[0.08121 1 0.1267] Hint UI Check
  (CallFunction|ToggleHintUI "" false))

(event Custom|BeginStartBloom
  (bind _startbloom (Timeline|StartBloom PlayFromStart)
    (:Update
      (Rendering|Material|SetScalarParameterValue "/Game/OuKanu/Materials/MP_Player.MP_Player" "StartBloom" _startbloom :!class /Script/Engine.KismetMaterialLibrary)
      (bind _floatmessage (Class|BPIPlayerController|GetFloatMessage(Message) (Pawn|GetController)))
      (UserInterface|SetWidget (Variables|Default|GetFloatMessageWidget) _floatmessage)
      (bind _hpbar (Class|BPIPlayerController|GetHPBar(Message) (Pawn|GetController)))
      (Variables|Default|SetHPBar _hpbar)
      (bind _output_get (Variables|Default|SetInitialCameraDistance (Variables|/Script/Engine.SpringArmComponent|GetTargetArmLength (Variables|Default|GetSpringArm))))
      (Variables|Default|SetCurrentCameraDis _output_get))))

(event EventBeginPlay
  (|CallParentFunction)
  (bind _startbloom (Timeline|StartBloom PlayFromStart)
    (:Update
      (Rendering|Material|SetScalarParameterValue "/Game/OuKanu/Materials/MP_Player.MP_Player" "StartBloom" _startbloom :!class /Script/Engine.KismetMaterialLibrary)
      (bind _floatmessage (Class|BPIPlayerController|GetFloatMessage(Message) (Pawn|GetController)))
      (UserInterface|SetWidget (Variables|Default|GetFloatMessageWidget) _floatmessage)
      (bind _hpbar (Class|BPIPlayerController|GetHPBar(Message) (Pawn|GetController)))
      (Variables|Default|SetHPBar _hpbar)
      (bind _output_get (Variables|Default|SetInitialCameraDistance (Variables|/Script/Engine.SpringArmComponent|GetTargetArmLength (Variables|Default|GetSpringArm))))
      (Variables|Default|SetCurrentCameraDis _output_get))))

(event Collision|EventActorBeginOverlap
  (params (OtherActor :type Actor%20Object%20Reference))
  (|CallParentFunction OtherActor) ; This node is disabled and will not be called.\nDrag off pins to build functionality.
)

(event EventTick
  (params (DeltaSeconds :type Float%20%28single-precision%29))
  (|CallParentFunction DeltaSeconds)
  (|SetCameraDisWithHP DeltaSeconds
    (:Output
      ;[1 1 1] WorldKillZ
      (if (<= (.z (Transformation|GetWorldLocation (Variables|Default|GetCapsuleComponent))) -1e+03)
        (CallFunction|Hurt 1e+04)))))

(event EventToggleHintUI
  (params (Text :type Text) (Enable :type Boolean))
  ;[0.08121 1 0.1267] Hint UI Check
  (bind _floatmessage (Class|BPIPlayerController|GetFloatMessage(Message) (Pawn|GetController)))
  (Class|BPIFloatUI|ShowText(Message) _floatmessage Text Enable))

(fn ConstructionScript
  (|CallParentFunction))

(fn IsPlayer
  (return (Pawn|IsPlayerControlled)))

(fn LostHPPercent
  (bind _hp_max (Variables|Default|GetHP_MAX))
  (return (/ (- _hp_max (Variables|Default|GetHP)) _hp_max)))

(fn UpdateHP
  (params (Damage :type Float%20%28single-precision%29))
  (|CallParentFunction Damage)
  (Class|BPIUI|SetHPBar(Message) (Variables|Default|GetHPBar) (/ (Variables|Default|GetHP) (Variables|Default|GetHP_MAX))))

(event EventPlayerReborn
  (bind _mesh (Variables|Character|GetMesh))
  (bind _mesh_2 (Variables|Character|GetMesh))
  (CallFunction|ResetAllInteractiveObjevt)
  ;[1 1 1] FadeScreen
  (bind _asrob_game_manager (Utilities|Casting|CastToRob_GameManager (Game|GetGameMode))
    (:then
      (Default|FadeOff _asrob_game_manager))
    (:CastFailed
      _))
  ;[1 1 1] DisableRagdoll
  (Transformation|SetWorldLocation (Variables|Default|GetCapsuleComponent) (Transformation|GetSocketLocation _mesh "root") false true)
  (Physics|SetSimulatePhysics _mesh false)
  (Collision|SetCollisionProfileName _mesh "CharacterMesh" :!class /Script/Engine.PrimitiveComponent)
  (Physics|SetSimulatePhysics _mesh false)
  (Collision|SetCollisionEnabled _mesh "NoCollision")
  (Physics|SetSimulatePhysics _mesh_2 false)
  (Transformation|AttachComponentToComponent _mesh_2 (Variables|Default|GetCapsuleComponent) "None" "KeepWorld" "KeepWorld" "KeepWorld" true)
  (Transformation|SetRelativeLocationAndRotation _mesh_2 "0, 0,-93.000000" "0,270.000000, 0" false true)
  (Variables|Default|SetCh_ActionState "NewEnumerator0")
  (Variables|Default|SetCanMove true)
  (CallFunction|Heal (Variables|Default|GetHP_MAX) true)
  (Variables|Default|SetImmune_Damage false)
  (bind _output_get (Variables|Default|SetDetathProcess 0.0))
  (Rendering|Material|SetScalarParameterValue "/Game/OuKanu/Materials/MP_Player.MP_Player" "DeathProcess" _output_get :!class /Script/Engine.KismetMaterialLibrary)
  (Variables|Default|SetStartBloom 0.0)
  (CallFunction|BeginStartBloom)
  (Variables|/Script/Engine.SpringArmComponent|SetTargetArmLength (Variables|Default|GetSpringArm) (Variables|Default|GetInitialCameraDistance))
  (CallFunction|ResetActor))

(event EventDeathProcess
  (bind _mesh (Variables|Character|GetMesh))
  (Utilities|FlowControl|DoOnce false :!label _label
    (:Completed
      (if (Utilities|Enum|Equal(Enum) (Variables|Default|GetCh_ActionState) "NewEnumerator3")
        (|UncrouchImmediate))
      (CallFunction|ResetAllInteractiveObjevt)
      (Variables|Default|SetCh_ActionState "NewEnumerator6")
      (Variables|Default|SetCanMove false)
      (Utilities|FlowControl|Sequence
        (:then_0
          ;[1 1 1] FadeScreenPostEffect
          (bind _deathprocess (Timeline|DeathScreenFade PlayFromStart)
            (:Update
              (bind _output_get (Variables|Default|SetDetathProcess _deathprocess))
              (Rendering|Material|SetScalarParameterValue "/Game/OuKanu/Materials/MP_Player.MP_Player" "DeathProcess" _output_get :!class /Script/Engine.KismetMaterialLibrary))))
        (:then_1
          ;[1 1 1] FadeScreenUI
          (bind _asrob_game_manager (Utilities|Casting|CastToRob_GameManager (Game|GetGameMode)))
          (Default|FadeON _asrob_game_manager))
        (:then_2
          (bind _returnvalue (Animation|PlayAnimMontage "/Game/OuKanu/Character/Main/Animations/Death/Standing_Death_Forward_02_Montage.Standing_Death_Forward_02_Montage" 1.0 "None"))
          (Utilities|FlowControl|RetriggerableDelay (* _returnvalue 0.5))
          ;[1 1 1] RagDoll
          (Collision|SetCollisionProfileName _mesh "Ragdoll" :!class /Script/Engine.PrimitiveComponent)
          (Physics|SetSimulatePhysics _mesh true)
          (Utilities|FlowControl|RetriggerableDelay (Math|Float|Max(Float) (- (Variables|Default|GetTotalDeathTime) (* _returnvalue 0.5)) 0.2))
          (Class|BPIPlayerController|RespawnPlayeratCheckPoint(Message) (Game|GetPlayerController 0))
          (goto _label Reset))))))